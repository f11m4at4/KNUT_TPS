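; BP_TPSGameMode is a game mode that tracks the current score and a persistent best score.
; On BeginPlay it creates the WBP_UIScreen widget and loads the saved best score from the BestScore slot if one exists.
; AddCurrentScore adds points and calls UpdateBestScore, which writes a new BP_SaveScore to that slot whenever the current score beats the best.
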(event EventBeginPlay
  (bind _returnvalue (UserInterface|CreateWidget "/Game/UI/WBP_UIScreen.WBP_UIScreen_C"))
  (Variables|Default|SetUIScreen _returnvalue)
  (bind _returnvalue_2 (SaveGame|DoesSaveGameExist "BestScore"))
  (if _returnvalue_2
    (bind _returnvalue_3 (SaveGame|LoadGamefromSlot "BestScore"))
    (bind _asbp_save_score (Utilities|Casting|CastToBP_SaveScore _returnvalue_3))
    (Variables|ScoreData|SetBestScore (Variables|/Game/Blueprints/BP_SaveScore.BP_SaveScore_C|GetBestScore _asbp_save_score))))

(event EventTick
  (params (DeltaSeconds :type Float%20%28single-precision%29)))

(fn ConstructionScript)

(fn AddCurrentScore
  (params (Point :type Integer))
  (Variables|ScoreData|SetCurrentScore (+ Point (Variables|ScoreData|GetCurrentScore)))
  (CallFunction|UpdateBestScore))

(fn UpdateBestScore
  (bind _currentscore (Variables|ScoreData|GetCurrentScore))
  (if (> _currentscore (Variables|ScoreData|GetBestScore))
    (Variables|ScoreData|SetBestScore _currentscore)
    (bind _returnvalue (SaveGame|CreateSaveGameObject "/Game/Blueprints/BP_SaveScore.BP_SaveScore_C"))
    (Variables|/Game/Blueprints/BP_SaveScore.BP_SaveScore_C|SetBestScore _returnvalue _currentscore)
    (SaveGame|SaveGametoSlot _returnvalue "BestScore")))