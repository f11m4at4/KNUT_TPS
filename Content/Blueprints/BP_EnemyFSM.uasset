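; Enemy AI state machine owned by BP_Enemy, targeting the BP_Player found at BeginPlay.
; Tick dispatches Idle, Move, Attack, Damage and Die states, with a shared timer driving delays; Move chases into range, while Attack only prints.
; OnDamageProcess decrements HP, then starts a timed lerp knockback or the Die state, which sinks the enemy downward.
; Two alternative knockback helpers, ToP0vt and ToLerp, are unused.
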(event EventTick
  (params (DeltaSeconds :type Float%20%28single-precision%29))
  (bind _mystate (Variables|Default|GetMyState))
  (Development|PrintString (Utilities|String|EnumtoString _mystate) false)
  (switch Utilities|FlowControl|Switch|SwitchonEEnemyState _mystate
    (:NewEnumerator0
      (CallFunction|IdleState))
    (:NewEnumerator1
      (CallFunction|MoveState))
    (:NewEnumerator2
      (CallFunction|AttackState))
    (:NewEnumerator3
      (CallFunction|DamageState))
    (:NewEnumerator4
      (CallFunction|DieState))))

(event EventBeginPlay
  ;[1 1 1] 월드에서 Player 타겟 찾아오기
  (bind _returnvalue (Actor|GetActorOfClass "/Game/Blueprints/BP_Player.BP_Player_C"))
  (Variables|Default|SetTarget _returnvalue)
  ;[1 1 1] 소유객체 가져오기
  (bind _asbp_enemy (Utilities|Casting|CastToBP_Enemy (Components|GetOwner)))
  (Variables|Default|SetMe _asbp_enemy))

(fn IdleState
  (bind _isfinish_ (CallFunction|FlowTime (Variables|Default|GetIdleDelayTime)))
  (if _isfinish_
    ;[1 1 1] 상태를 이동으로 전환하기
    (Variables|Default|SetMyState "NewEnumerator1")))

(fn MoveState
  (bind _target (Variables|Default|GetTarget))
  (bind _me (Variables|Default|GetMe))
  (bind _returnvalue (Transformation|GetActorLocation _me))
  (bind _returnvalue_2 (Transformation|GetActorLocation _target))
  (bind _returnvalue_3 (- _returnvalue_2 _returnvalue))
  ;[1 1 1] 타겟방향구하기
  (LocalVariables|SetDistance (Math|Vector|VectorLength _returnvalue_3))
  (bind _output_get (LocalVariables|SetDirection (Math|Vector|Normalize _returnvalue_3)))
  ;[1 1 1] 이동하고싶다.
  (Pawn|Input|AddMovementInput (Variables|Default|GetMe) _output_get 1.0 false)
  ;[1 1 1] 공격상태 전환 체크
  (if (< (LocalVariables|GetDistance) (Variables|Default|GetAttackRange))
    (Variables|Default|SetMyState "NewEnumerator2")))

(fn AttackState
  ;[1 1 1] 일정시간에 한번씩 공격하기
  (bind _isfinish_ (CallFunction|FlowTime (Variables|Default|GetAttackDelayTime)))
  (if _isfinish_
    (Development|PrintString "공격!!!!")
    ;[1 1 1] 공격범위를 벗어났을 때 상태를 이동으로 전환
    (if (> (Math|Vector|Distance(Vector) (Transformation|GetActorLocation (Variables|Default|GetTarget)) (Transformation|GetActorLocation (Variables|Default|GetMe))) (Variables|Default|GetAttackRange))
      (Variables|Default|SetMyState "NewEnumerator1"))))

(fn DamageState
  (if (Variables|Default|GetNuckbackPlaying)
    (CallFunction|Nuckback))
  ;[1 1 1] 일정시간후에 대기상태로 전환
  (bind _isfinish_ (CallFunction|FlowTime (Variables|Default|GetDamageDelayTime)))
  (if _isfinish_
    (Variables|Default|SetMyState "NewEnumerator0")))

(fn DieState
  (Transformation|SetActorLocation (Variables|Default|GetMe) (+ (Transformation|GetActorLocation (Variables|Default|GetMe)) (* (* (Math|Vector|VectorDown) (Variables|Default|GetDieSpeed)) (Utilities|Time|GetWorldDeltaSeconds))) false false))

(fn FlowTime
  (params (DelayTime :type Float%20%28double-precision%29))
  ;[1 1 1] 시간이 흐른다.
  (bind _output_get (Variables|Default|SetCurrentTime (+ (Variables|Default|GetCurrentTime) (Utilities|Time|GetWorldDeltaSeconds))))
  ;[1 1 1] 대기시간을 초과했다면
  (if (> _output_get DelayTime)
    (Variables|Default|SetCurrentTime 0.0)
    (return true)
    (else
      (return false))))

(fn OnDamageProcess
  (params (HitDirection :type Vector :default "1.000000,0.000000,0.000000"))
  (Variables|Default|SetHit%20Direction HitDirection)
  (Variables|Default|SetCurrentTime 0.0)
  ;[1 1 1] 체력 감소
  (bind _result (Math|Integer|DecrementInt (Variables|Default|GetHP))
    (:%20%20
      (if (> _result 0)
        (Variables|Default|SetMyState "NewEnumerator3")
        (Variables|Default|SetNuckbackPlaying true)
        (bind _output_get (Variables|Default|SetStartPoint (Transformation|GetActorLocation (Variables|Default|GetMe))))
        (Variables|Default|SetEndPoint (+ _output_get (* (Variables|Default|GetHit%20Direction) (Variables|Default|GetNuckbackDistance))))
        (Variables|Default|SetNuckbackTime 0.0)
        (else
          (Variables|Default|SetMyState "NewEnumerator4"))))))

(fn Nuckback
  ;[1 1 1] 넉백
  (Transformation|SetActorLocation (Variables|Default|GetMe) (CallFunction|ToTimeRange) true false)
  (if (< (Math|Vector|Distance(Vector) (Transformation|GetActorLocation (Variables|Default|GetMe)) (Variables|Default|GetEndPoint)) (Variables|Default|GetNuckbackStopRange))
    (Transformation|SetActorLocation (Variables|Default|GetMe) (Variables|Default|GetEndPoint) false false)
    (Variables|Default|SetNuckbackPlaying false)))

(fn ToP0vt
  (return (+ (* (* (Variables|Default|GetHit%20Direction) (Variables|Default|GetNuckbackPower)) (Utilities|Time|GetWorldDeltaSeconds)) (Transformation|GetActorLocation (Variables|Default|GetMe)))))

(fn ToLerp
  (return (Math|Vector|Lerp(Vector) (Transformation|GetActorLocation (Variables|Default|GetMe)) (Variables|Default|GetEndPoint) (* (Variables|Default|GetNuckbackPower) (Utilities|Time|GetWorldDeltaSeconds)))))

(fn ToTimeRange
  (Variables|Default|SetNuckbackTime (+ (Variables|Default|GetNuckbackTime) (Utilities|Time|GetWorldDeltaSeconds)))
  (return (Math|Vector|Lerp(Vector) (Variables|Default|GetStartPoint) (Variables|Default|GetEndPoint) (Math|Float|Clamp(Float) (/ (Variables|Default|GetNuckbackTime) (Variables|Default|GetNuckbackFinishTime))))))